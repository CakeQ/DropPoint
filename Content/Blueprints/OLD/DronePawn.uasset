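; Player-controlled drone pawn that moves, dodges sideways, shoots and is destroyed when its health runs out.
; Movement follows control rotation, while the mesh eases toward look input, with a movement-based turning branch gated by lock target and recent look activity.
; Holding the trigger spawns the ammo class at the barrel, rate-limited by that class's default cooldown.
; Dodges are forced left or right movement inputs.
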(event `InputAction|DodgeRight`
  (params (Key :type "Key Structure"))
  (:`Pressed`
    (`self.Dodge` true)))

(event `InputAction|DodgeLeft`
  (params (Key :type "Key Structure"))
  (:`Pressed`
    (`self.Dodge` false)))

(event `InputAxis|LookX`
  (params (AxisValue :type "Float (single-precision)"))
  (bind _mesh (`self.Mesh`))
  (bind _returnvalue (`SceneComponent.K2_GetComponentLocation` _mesh))
  (if (!= AxisValue 0.0)
    (`SceneComponent.K2_SetWorldRotation` _mesh (`KismetMathLibrary.RInterpTo` (`SceneComponent.K2_GetComponentRotation` _mesh) (`KismetMathLibrary.FindLookAtRotation` _returnvalue (+ _returnvalue (`KismetMathLibrary.MakeVector` (* (stale `InputAxis|LookY` AxisValue) -100.0) (* AxisValue 100.0)))) (stale `self.ReceiveTick` DeltaSeconds) 4.0) false false :!label _label)
    (set `self.lastMouseMoved` (`KismetSystemLibrary.GetGameTimeInSeconds`))))

(event `InputAxis|LookY`
  (params (AxisValue :type "Float (single-precision)"))
  (if (!= AxisValue 0.0)
    (goto _label)))

(event `InputAxis|MoveY`
  (params (AxisValue :type "Float (single-precision)"))
  (bind _mesh (`self.Mesh`))
  (bind _returnvalue (`SceneComponent.K2_GetComponentLocation` _mesh))
  (if (!= AxisValue 0.0)
    (`self.AddMovementInput` (`KismetMathLibrary.GetForwardVector` (`self.GetControlRotation`)) AxisValue)
    (if (and (not (or (`KismetSystemLibrary.IsValid` (`self.LockTarget`)) (or (!= (stale `InputAxis|LookX` AxisValue) 0.0) (!= (stale `InputAxis|LookY` AxisValue) 0.0)))) (<= (+ (`self.lastMouseMoved`) 1.0) (`KismetSystemLibrary.GetGameTimeInSeconds`))) :!label _label_2
      (`SceneComponent.K2_SetWorldRotation` _mesh (`KismetMathLibrary.RInterpTo` (`SceneComponent.K2_GetComponentRotation` _mesh) (`KismetMathLibrary.FindLookAtRotation` _returnvalue (+ _returnvalue (`KismetMathLibrary.MakeVector` (* AxisValue 100.0) (* (stale `InputAxis|MoveX` AxisValue) 100.0)))) (stale `self.ReceiveTick` DeltaSeconds) 4.0) false false))))

(event `InputAxis|MoveX`
  (params (AxisValue :type "Float (single-precision)"))
  (if (!= AxisValue 0.0)
    (`self.AddMovementInput` (`KismetMathLibrary.GetRightVector` (`self.GetControlRotation`)) AxisValue)
    (goto _label_2)))

(event `self.ReceiveTick`
  (params (DeltaSeconds :type "Float (single-precision)")))

(event `InputAxis|TriggerHeld`
  (params (AxisValue :type "Float (single-precision)"))
  (bind _ammotype (`self.AmmoType`))
  (if (and (== AxisValue 1.0) (> (`KismetSystemLibrary.GetGameTimeInSeconds`) (+ (`self.LastFired`) (`.Cooldown` (defaults `Object` _ammotype)))))
    (`|SpawnActorFromClass` _ammotype (`KismetMathLibrary.MakeTransform` (.location (`SceneComponent.K2_GetComponentToWorld` (`self.Barrel`))) (.rotation (`SceneComponent.K2_GetComponentToWorld` (`self.Barrel`))) (.scale (`SceneComponent.K2_GetComponentToWorld` (`self.Barrel`)))) "Undefined" "OverrideRootScale" self null)
    (set `self.LastFired` (`KismetSystemLibrary.GetGameTimeInSeconds`))))

(fn `Die`
  (`self.K2_DestroyActor`))

(fn `Dodge`
  (params (Right :type Boolean))
  (bind _returnvalue (`KismetMathLibrary.GetRightVector` (`self.GetControlRotation`)))
  (if Right
    (`self.AddMovementInput` _returnvalue 1.0 true)
    (else
      (`self.AddMovementInput` _returnvalue -1.0 true))))

(fn `TakeDamage`
  (params (Damage :type Integer :default 1))
  (bind _output_get (set `self.Health` (- (`self.Health`) Damage)))
  (if (<= _output_get 0)
    (`self.Die`)))

(fn `UserConstructionScript`)