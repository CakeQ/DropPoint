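; Test actor that previews a unit landing effect with a Niagara component and an animated skeletal mesh.
; On BeginPlay it plays a timeline and checks the track value on every update.
; Values near zero restart the Niagara system, while values near one rewind the mesh animation to its start with notifies enabled.
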(event `self.ReceiveBeginPlay`
  (bind (_direction _newtrack_0) (`Timeline|Timeline_0`)
    (:`Update`
      (if (`KismetMathLibrary.NearlyEqual_FloatFloat` _newtrack_0 0.0 0.1)
        (`ActorComponent.Deactivate` (`self.Niagara`))
        (`ActorComponent.Activate` (`self.Niagara`) false)
        (elif (`KismetMathLibrary.NearlyEqual_FloatFloat` _newtrack_0 1.0 0.1)
          (`SkeletalMeshComponent.SetPosition` (`self.SkeletalMesh`) 0.0 true))))))

(fn `UserConstructionScript`)