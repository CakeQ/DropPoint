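; Bullet is a projectile actor that damages drone pawns on overlap.
; Each tick it offsets itself along its root component's forward vector by Speed, without sweeping or delta-time scaling, and destroys itself once its Lifespan is exceeded.
; Overlapping any actor other than its owner also destroys it, first passing Damage to TakeDamage if that actor is a DronePawn.
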(event `self.ReceiveActorBeginOverlap`
  (params (OtherActor :type "Actor Object Reference"))
  (if (!= OtherActor (`self.GetOwner`))
    (bind _asdrone_pawn (cast `/Game/Blueprints/DronePawn` OtherActor)
      (:`then`
        (`/Game/Blueprints/DronePawn.TakeDamage` _asdrone_pawn (`self.Damage`)))
      (:`CastFailed`
        _))
    (`self.K2_DestroyActor`)))

(event `self.ReceiveTick`
  (params (DeltaSeconds :type "Float (single-precision)"))
  (`self.K2_AddActorWorldOffset` (* (`SceneComponent.GetForwardVector` (`self.DefaultSceneRoot`)) (`self.Speed`)))
  (if (> (`self.GetGameTimeSinceCreation`) (`self.Lifespan`))
    (`self.K2_DestroyActor`)))

(fn `UserConstructionScript`)